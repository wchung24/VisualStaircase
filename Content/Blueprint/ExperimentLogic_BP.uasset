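; Experiment logic Blueprint for what appears to be a camera-movement perception test, where gamepad triggers record whether the participant claims movement.
; Each tick appends camera yaw divided by delta time to an array and rewrites it to a DATA file at a hard-coded path.
; Tick also loops a yaw-versus-claim check while its flag holds, and advances on-screen triplet counters independently of that result.
; The incorrect-answer counter is never called, and the timestamped log name is unused.
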(event `self.ReceiveBeginPlay`
  (set `self.NameOfLogFile` (`KismetStringLibrary.Concat_StrStr` (`KismetStringLibrary.Conv_IntToString` (`KismetMathLibrary.GetDays` (struct))) (`KismetStringLibrary.Concat_StrStr` (`KismetStringLibrary.Concat_StrStr` (`KismetStringLibrary.Conv_IntToString` (`KismetMathLibrary.GetHours` (struct))) ":") (`KismetStringLibrary.Conv_IntToString` (`KismetMathLibrary.GetMinutes` (struct)))))))

(event `UpdateLogFile`
  (bind _arrayofr_velocities (`self.ArrayOfR_Velocities`))
  (bind (_returnvalue_roll _returnvalue_pitch _returnvalue_yaw) (`KismetMathLibrary.BreakRotator` (`PlayerCameraManager.GetCameraRotation` (`GameplayStatics.GetPlayerCameraManager` 0))))
  (bind _returnvalue (`KismetStringLibrary.Conv_DoubleToString` (/ _returnvalue_yaw (`GameplayStatics.GetWorldDeltaSeconds`))))
  (bind _result (`/Engine/EditorBlueprintResources/StandardMacros.IncrementInt` (`self.ArrayIndex`))
    (:`  `
      (`KismetSystemLibrary.PrintString` _returnvalue true true (struct :`G` 0.66 :`B` 1.0 :`A` 1.0) 0.0)
      (`KismetArrayLibrary.Array_Set` _arrayofr_velocities _result _returnvalue true)
      (`VictoryBPFunctionLibrary.FileIO__SaveStringArrayToFile` "C:\\Users\\labadmin\\Documents\\Unreal Projects\\PythonTest2\\Content" "DATA" _arrayofr_velocities true))))

(event `CorrectUntil`
  (bind (_returnvalue_roll _returnvalue_pitch _returnvalue_yaw) (`KismetMathLibrary.BreakRotator` (`PlayerCameraManager.GetCameraRotation` (`GameplayStatics.GetPlayerCameraManager` 0))))
  (if (and (> _returnvalue_yaw 0.0) (`self.ParticipantClaimsMovement`))
    ;[1 1 1] If answered Correct
    (set `self.CorrectUntilBool` true)
    (else
      ;[1 1 1] If answered Incorrect
      (set `self.CorrectUntilBool` false))))

(event `self.ReceiveTick`
  (params (DeltaSeconds :type "Float (single-precision)"))
  (`self.UpdateLogFile`)
  (while (`self.CorrectUntilBool`)
    (`self.CorrectUntil`))
  (if (< (`self.Total3InARow`) 3)
    (`self.AddToTriplet`)
    (else
      (set `self.Total3InARow` 0)
      (if (< (`self.TotalTriplets`) 5)
        (`self.TripletsTotal`)))))

(event `AddToTriplet`
  (bind _result (`/Engine/EditorBlueprintResources/StandardMacros.IncrementInt` (`self.Total3InARow`))
    (:`  `
      (`TextRenderComponent.K2_SetText` (`self.TripletsInARow`) (`KismetTextLibrary.Conv_IntToText` _result)))))

(event `Key|Gamepad_RightTrigger`
  (params (Key :type "Key Structure"))
  (:`Pressed`
    (set `self.ParticipantClaimsMovement` true)))

(event `Key|Gamepad_LeftTrigger`
  (params (Key :type "Key Structure"))
  (:`Pressed`
    (set `self.ParticipantClaimsMovement` false)))

(event `TripletsTotal`
  (bind _result (`/Engine/EditorBlueprintResources/StandardMacros.IncrementInt` (`self.TotalTriplets`))
    (:`  `
      (`TextRenderComponent.K2_SetText` (`self.TotalTripletz`) (`KismetTextLibrary.Conv_IntToText` _result)))))

(event `TotalIncorrectAnswers`
  (bind _result (`/Engine/EditorBlueprintResources/StandardMacros.IncrementInt` (`self.TotalIncorrect`))
    (:`  `
      (`TextRenderComponent.K2_SetText` (`self.TotalWrong`) (`KismetTextLibrary.Conv_IntToText` _result)))))

(fn `UserConstructionScript`)